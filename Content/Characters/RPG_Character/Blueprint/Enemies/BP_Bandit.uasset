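; BP_Bandit is an RPG enemy character that defines the starting stats for a Bandit.
; On BeginPlay it calls InitStats, which writes team, name and max health to the BPCEntities component and starts health at that maximum.
; Overlap and Tick are disabled stubs, so the Blueprint adds no behavior beyond this setup.
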(event `self.ReceiveBeginPlay`
  (`self.InitStats`))

(fn `InitStats`
  (`self.InitStats_0`))

(fn `InitStats_0`
  (bind _bpc_entities (`self.BPC_Entities`))
  (set `/Game/Characters/RPG_Character/Blueprint/BPC_Entities.Team` "NewEnumerator2" _bpc_entities)
  (bind _output_get (set `/Game/Characters/RPG_Character/Blueprint/BPC_Entities.MaxHealth` 50.0 _bpc_entities))
  (set `/Game/Characters/RPG_Character/Blueprint/BPC_Entities.Health` _output_get _bpc_entities)
  (set `/Game/Characters/RPG_Character/Blueprint/BPC_Entities.Name` "Bandit" _bpc_entities))

(fn `UserConstructionScript`
  (`parent.UserConstructionScript`))